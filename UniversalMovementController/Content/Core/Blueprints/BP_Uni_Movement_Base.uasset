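; Base movement character Blueprint that provides Enhanced Input movement, camera look and a timed speed boost, registering IMC_Main on BeginPlay.
; Move input follows control rotation unless movement is disallowed.
; Boolean options select how look input drives the controller, spring arm, follow camera and orient-to-movement setting.
; Boost swaps MaxWalkSpeed between boost and normal values, with a DoOnce and delays enforcing duration and recharge, reported through debug prints.
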(event Input|EnhancedActionEvents|EnhancedInputActionIA_WASD-Move
  (params (ActionValue :type Vector%202D%20Structure) (ElapsedSeconds :type Float%20%28double-precision%29) (TriggeredSeconds :type Float%20%28double-precision%29) (InputAction :type Input%20Action%20Object%20Reference :default "/Game/Core/Input/IA/IA_WASD-Move.IA_WASD-Move"))
  (bind _returnvalue (Pawn|GetControlRotation :!class /Script/Engine.Pawn))
  ;[0 0 0] Movement -WASD
  (if (Variables|AstersAttributes|GetDisallow%20Movement)
    (Variables|AstersAttributes|SetDisallow%20Movement true)
    (else
      (Variables|AstersAttributes|SetDisallow%20Movement false)
      (Pawn|Input|AddMovementInput (Math|Vector|GetRightVector (Math|Rotator|MakeRotator (.roll _returnvalue) 0.0 (.yaw _returnvalue))) (.x ActionValue) false)
      (Pawn|Input|AddMovementInput (Math|Vector|GetForwardVector (Math|Rotator|MakeRotator 0.0 0.0 (.yaw _returnvalue))) (.y ActionValue) false))))

(event Input|EnhancedActionEvents|EnhancedInputActionIA_Boost
  (params (ActionValue :type Boolean) (ElapsedSeconds :type Float%20%28double-precision%29) (TriggeredSeconds :type Float%20%28double-precision%29) (InputAction :type Input%20Action%20Object%20Reference :default "/Game/Core/Input/IA/IA_Boost.IA_Boost"))
  ;[0 0 0] Speed Boost Logic
  (if (Variables|AstersAttributes|GetBoost%20Allowed)
    (Variables|AstersAttributes|SetBoost%20Allowed true)
    (Utilities|FlowControl|DoOnce false :!label _label
      (:Completed
        (CallFunction|StartBoost)
        ;;[0 0 0] Boost Time (In Seconds)
        (Utilities|FlowControl|Delay 5.0)
        (CallFunction|StopBoost)
        (Development|PrintString "Recharging Boost" true true "(R=1.000000,G=0.009744,B=0.000000,A=1.000000)" 5.0)
        ;;[0 0 0] Boost Recharge Time (In Seconds)
        (Utilities|FlowControl|Delay 5.0)
        (goto _label Reset)))
    (else
      (Variables|AstersAttributes|SetBoost%20Allowed false))))

(event Input|EnhancedActionEvents|EnhancedInputActionIA_Camera-Move
  (params (ActionValue :type Vector%202D%20Structure) (ElapsedSeconds :type Float%20%28double-precision%29) (TriggeredSeconds :type Float%20%28double-precision%29) (InputAction :type Input%20Action%20Object%20Reference :default "/Game/Core/Input/IA/IA_Camera-Move.IA_Camera-Move"))
  (bind _followcamera (Variables|Default|GetFollowCamera))
  (bind _charactermovement (Variables|Character|GetCharacterMovement))
  ;[0 0 0] Camera setup
  (if (Variables|AstersAttributes|GetOrient%20Rotation%20to%20Movement%20Direction)
    (Variables|AstersAttributes|SetOrient%20Rotation%20to%20Movement%20Direction true)
    (Variables|Default|SetbUseControllerRotationYaw false)
    (Pawn|Input|AddControllerYawInput 0.0)
    (if (Variables|AstersAttributes|GetAllow%20Camera%20Rotation%20Control)
      (Variables|/Script/Engine.CharacterMovementComponent|SetbOrientRotationToMovement _charactermovement true)
      (Variables|AstersAttributes|SetAllow%20Camera%20Rotation%20Control true)
      (else
        (Variables|/Script/Engine.CharacterMovementComponent|SetbOrientRotationToMovement _charactermovement false)
        (Variables|AstersAttributes|SetAllow%20Camera%20Rotation%20Control true)))
    (elif (Variables|AstersAttributes|GetUse%20Pawn%20Rotation)
      (if (Variables|AstersAttributes|GetUse%20Pawn%20Rotation)
        (Variables|AstersAttributes|SetAllow%20Camera%20Rotation%20Control true)
        (Variables|AstersAttributes|SetUse%20Pawn%20Rotation true)
        (Pawn|Input|AddControllerYawInput (.x ActionValue))
        (Pawn|Input|AddControllerPitchInput (.y ActionValue))
        ;;[0 0 0] Camera Details panel Options
        (Variables|/Script/Engine.SpringArmComponent|SetbUsePawnControlRotation (Variables|Default|GetCamera_Boom) true)
        (if (Variables|AstersAttributes|GetLock%20camera%20ROTATION%20but%20allow%20Look%20Up%20down)
          (Variables|/Script/Engine.CameraComponent|SetbUsePawnControlRotation _followcamera (Variables|/Script/Engine.CameraComponent|GetbUsePawnControlRotation _followcamera))
          (Variables|/Script/Engine.CameraComponent|SetbUsePawnControlRotation _followcamera true)
          (Variables|/Script/Engine.SpringArmComponent|SetbUsePawnControlRotation (Variables|Default|GetCamera_Boom) false))
        (else
          (Variables|AstersAttributes|SetUse%20Pawn%20Rotation false)))
      (elif (Variables|AstersAttributes|GetAllow%20Camera%20Rotation%20Control)
        (Variables|AstersAttributes|SetAllow%20Camera%20Rotation%20Control true)
        (Pawn|Input|AddControllerYawInput (.x ActionValue))
        (Pawn|Input|AddControllerPitchInput (.y ActionValue))
        (else
          (Variables|AstersAttributes|SetAllow%20Camera%20Rotation%20Control false))))))

(event EventBeginPlay
  ;[0 0 0] Cast to and find controllers
  (bind _asplayer_controller (Utilities|Casting|CastToPlayerController (Pawn|GetController)))
  (Utilities|IsValid (PlayerController|LocalPlayerSubsystems|GetEnhancedInputLocalPlayerSubsystem _asplayer_controller)
    (:Is%20Valid
      (Input|AddMappingContext (PlayerController|LocalPlayerSubsystems|GetEnhancedInputLocalPlayerSubsystem _asplayer_controller) "/Game/Core/Input/Context/IMC_Main.IMC_Main" 0 "(bIgnoreAllPressedKeysUntilRelease=True,bForceImmediately=False,bNotifyUserSettings=False)"))))

(fn ConstructionScript)

(fn StartBoost
  (Development|PrintString "Boost started")
  (Variables|/Script/Engine.CharacterMovementComponent|SetMaxWalkSpeed (Variables|Character|GetCharacterMovement) (Variables|AstersAttributes|GetBoost%20Speed))
  (Development|PrintString "Boosting ( Active )" true true "(R=1.000000,G=0.000000,B=0.008162,A=1.000000)" 5.0))

(fn StopBoost
  (Development|PrintString "Out of Boost Energy" true true "(R=0.000000,G=0.660000,B=1.000000,A=1.000000)" 2.5)
  (Variables|/Script/Engine.CharacterMovementComponent|SetMaxWalkSpeed (Variables|Character|GetCharacterMovement) (Variables|AstersAttributes|GetNormal%20Speed))
  (Development|PrintString "Boost ( In-Active ) Until Recharge in 5 Seconds" true true "(R=0.000000,G=0.660000,B=1.000000,A=1.000000)" 3.0))